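; EventTrigger_BP is a trigger actor that adds a new event to a chosen timeline when anything begins overlapping its box.
; On overlap it fetches the timeline and, if valid, creates an event from the configured class, name, duration and delay.
; The construction script gives the cube a dynamic material and, when the timeline has a mapped color, tints it and writes these settings to a text label.
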(event OnComponentBeginOverlap(Box)
  (params (OverlappedComponent :type Primitive%20Component%20Object%20Reference) (OtherActor :type Actor%20Object%20Reference) (OtherComp :type Primitive%20Component%20Object%20Reference) (OtherBodyIndex :type Integer) (bFromSweep :type Boolean) (SweepResult :type Hit%20Result%20Structure%20%28by%20ref%29))
  (bind _timeline (Variables|EventsConfiguration|GetTimeline))
  (bind _returnvalue (Class|NTimelineBlueprintHelpers|GetTimeline _timeline))
  (Utilities|IsValid _returnvalue
    (:Is%20Valid
      (Class|NTimelineManagerDecorator|CreateandAddNewEvent _returnvalue (Variables|EventsConfiguration|GetName) (Variables|EventsConfiguration|GetEvents) (Variables|EventsConfiguration|GetDuration) (Variables|EventsConfiguration|GetDelay)))))

(fn ConstructionScript
  (bind _colorfortimeline (Variables|Default|GetColorForTimeline))
  (bind _timeline (Variables|EventsConfiguration|GetTimeline))
  (bind (_value _returnvalue) (Utilities|Map|Find _colorfortimeline _timeline))
  (bind _returnvalue_2 (Rendering|Material|CreateDynamicMaterialInstance (Variables|Default|GetCube) 0 "/Game/Material/Mat_Trigger.Mat_Trigger" "None" :!class /Script/Engine.PrimitiveComponent))
  (if _returnvalue
    (Rendering|Material|SetVectorParameterValue _returnvalue_2 "Color" _value :!class /Script/Engine.MaterialInstanceDynamic)
    (Rendering|Components|TextRender|SetText (Variables|Default|GetTextRender) (Utilities|Text|ToText(String) (Utilities|String|Append "Timeline: " (Utilities|String|ToString(Name) (Class|NTimelineBlueprintHelpers|GetName _timeline)) " 
 Events class: " (Utilities|GetClassDisplayName (Variables|EventsConfiguration|GetEvents)) " 
Duration: " (Utilities|String|ToString(Float) (Variables|EventsConfiguration|GetDuration)) " 
Delay: " (Utilities|String|ToString(Float) (Variables|EventsConfiguration|GetDelay)) " 
Name: " (Utilities|String|ToString(Name) (Variables|EventsConfiguration|GetName)))))))